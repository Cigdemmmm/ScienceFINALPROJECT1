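; BP_AI is a sword-and-shield enemy character that spots, attacks and takes damage from the third-person player.
; Pawn sensing sets a Blackboard seen flag, caches the player and AI controller, and binds to the player's hit dispatcher.
; Hits reduce health only after a sphere overlap sets IsNear, report it back to the player, and on death stop AI logic.
; AttackPlayer sphere-traces ahead to play a slash montage; sword overlap damages the player.
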(event OnSeePawn(PawnSensing)
  (params (Pawn :type Pawn%20Object%20Reference))
  (bind _asbp_third_person_character (Utilities|Casting|CastToBP_ThirdPersonCharacter Pawn))
  (AI|Components|Blackboard|SetValueasBool (AI|GetBlackboard (AI|GetAIController self)) (Utilities|Name|MakeLiteralName "Seentarget?") true)
  (bind _output_get (Variables|Default|SetAs%20BP%20Third%20Person%20Character _asbp_third_person_character))
  (EventDispatchers|AssignDPHit _output_get (delegate Custom|DP_Hit_Event))
  (bind _asbp_aicontroller (Utilities|Casting|CastToBP_AIController (Pawn|GetController)))
  (Variables|Default|SetAs%20BP%20AIController _asbp_aicontroller))

(event OnComponentBeginOverlap(Sword)
  (params (OverlappedComponent :type Primitive%20Component%20Object%20Reference) (OtherActor :type Actor%20Object%20Reference) (OtherComp :type Primitive%20Component%20Object%20Reference) (OtherBodyIndex :type Integer) (bFromSweep :type Boolean) (SweepResult :type Hit%20Result%20Structure%20%28by%20ref%29))
  (bind _as_bp_third_person_character (Variables|Default|GetAs%20BP%20Third%20Person%20Character))
  (if (== OtherActor _as_bp_third_person_character)
    (Default|HealthUpdate _as_bp_third_person_character -1e+01)))

(event OnComponentBeginOverlap(Sphere)
  (params (OverlappedComponent :type Primitive%20Component%20Object%20Reference) (OtherActor :type Actor%20Object%20Reference) (OtherComp :type Primitive%20Component%20Object%20Reference) (OtherBodyIndex :type Integer) (bFromSweep :type Boolean) (SweepResult :type Hit%20Result%20Structure%20%28by%20ref%29))
  (Variables|Default|SetIsNear? true))

(event Custom|AttackPlayer
  (bind _returnvalue (Transformation|GetActorLocation))
  (bind (_outhit _returnvalue_2) (Collision|SphereTraceForObjects _returnvalue (+ _returnvalue (* (Math|Vector|GetForwardVector (Transformation|GetActorRotation)) 1e+01)) 1.2e+02 (Utilities|Array|MakeArray "ObjectTypeQuery3") false 0 "None"))
  (if _returnvalue_2
    (Utilities|Casting|CastToBP_ThirdPersonCharacter (.HitActor (Collision|BreakHitResult _outhit)))
    (Animation|PlayAnimMontage "/Game/Final/AI/Attack/Sword_And_Shield_Slash_Montage.Sword_And_Shield_Slash_Montage" 1.0 "None")))

(event Custom|DP_Hit_Event
  (bind _as_bp_aicontroller (Variables|Default|GetAs%20BP%20AIController))
  (if (Variables|Default|GetIsNear?)
    (bind _output_get (Variables|Default|SetHealth (- (Variables|Default|GetHealth) 5.0)))
    (Default|CallDPEnemyHealthUpdate (Variables|Default|GetAs%20BP%20Third%20Person%20Character) _output_get)
    (if (<= _output_get 0.0)
      (Variables|Default|SetIsNear? false)
      (AI|Logic|StopLogic (Variables|/Script/AIModule.AIController|GetBrainComponent _as_bp_aicontroller) "")
      (AI|Navigation|StopMovement _as_bp_aicontroller)
      (Components|Animation|PlayAnimation (Variables|Character|GetMesh) "/Game/Final/AI/Attack/Sword_And_Shield_Death.Sword_And_Shield_Death" false)
      (Collision|SetCollisionEnabled (Variables|Character|GetMesh) "NoCollision"))))

(event Collision|EventActorBeginOverlap
  (params (OtherActor :type Actor%20Object%20Reference)))

(event EventTick
  (params (DeltaSeconds :type Float%20%28single-precision%29)))

(fn ConstructionScript)

(fn SwordAttack
  (bind _returnvalue (Animation|PlayAnimMontage "/Game/Final/AI/Attack/AM_AttackMontage.AM_AttackMontage" 1.0 "None"))
  (return _returnvalue))